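; Actor that drives a skeletal mesh through a Control Rig using pose data streamed from a local TCP server.
; BeginPlay retries the connection on a looping timer until it succeeds, and EndPlay closes the socket.
; Each tick reads the pose data and sets each control's scaled location, with a hardcoded rotation for head, hands and feet.
; When no data arrives, a timeout timer closes the socket and restarts the reconnect loop.
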(event OnPreInitializeDelegate(ControlRig)
  (params (Component :type Control%20Rig%20Component%20Object%20Reference))
  (Class|ControlRigComponent|AddMappedCompleteSkeletalMesh Component (Variables|Default|GetSkeletalMesh) "Output") ; Apply Skeletal mesh to control rig
)

(event Custom|TCPTimedout
  (CallFunction|CloseTCP (Variables|Default|GetTCPSocket))
  (Variables|Default|SetTCPConnected false) ; Reset status to disconnected, then reattempt to connect
  (bind _returnvalue (Utilities|Time|SetTimerbyEvent (delegate Custom|Connect%20TCP) 3.0 true false -3.0)) ; Attempt to connect to TCP server on a loop using a timer
  (bind _output_get (Variables|Default|SetTCPConnecting _returnvalue)))

(event Custom|Connect%20TCP
  (bind (_success _socket) (CallFunction|ConnectTCP "127.0.0.1" 15815))
  (if _success
    (Variables|Default|SetTCPSocket _socket)
    (Variables|Default|SetTCPConnected true)
    (Utilities|Time|ClearandInvalidateTimerbyHandle (stale Custom|TCPTimedout _output_get)) ; Successfully connected, stop further attempts
    (else
      (Development|PrintText "Retrying in 3 seconds..."))))

(event EventEndPlay
  (params (EndPlayReason :type EEndPlayReason%20Enum :default "Destroyed"))
  (CallFunction|CloseTCP (Variables|Default|GetTCPSocket))
  (Variables|Default|SetTCPConnected false))

(event EventBeginPlay
  (bind _returnvalue (Utilities|Time|SetTimerbyEvent (delegate Custom|Connect%20TCP) 3.0 true false -3.0)) ; Attempt to connect to TCP server on a loop using a timer
  (bind _output_get (Variables|Default|SetTCPConnecting _returnvalue)))

(event EventTick
  (params (DeltaSeconds :type Float%20%28single-precision%29))
  (bind (_returnvalue _posedata) (CallFunction|TCPTick (Variables|Default|GetTCPConnected) (Variables|Default|GetTCPSocket) (Variables|Default|GetTCPTimeout))) ; Returns 0 on success, 1 on no data, 2 on no connection
  (Math|Integer|CompareInt _returnvalue 1 ; Read return value
    (:==
      (if (not (Class|KismetSystemLibrary|TimerExistsHandle (Variables|Default|GetTCPTimeout)))
        (bind _returnvalue_2 (Utilities|Time|SetTimerbyEvent (delegate Custom|TCPTimedout) 5.0)) ; Timer to call TCPTimedout
        (Variables|Default|SetTCPTimeout _returnvalue_2) ; No data, set timeout if no previous timeout timer exist
      ))
    (:<
      (bind _keys (Utilities|Map|Keys _posedata)) ; Read pose data
      (for _array_element _keys
        (switch name (Utilities|String|StringToName _array_element)
          (:Default
            (Variables|Default|SetcurrentRotation "0, 0, 0"))
          (:head_ctrl
            (bind _output_get (Variables|Default|SetcurrentRotation "90.000000,0.000000,0.000000" :!label _label)))
          (:hand_l_ctrl
            (Variables|Default|SetcurrentRotation "-90.000000,0.000000,0.000000"))
          (:hand_r_ctrl
            (Variables|Default|SetcurrentRotation "90.000000,180.000000,0.000000"))
          (:foot_l_ctrl
            (goto _label))
          (:foot_r_ctrl
            (Variables|Default|SetcurrentRotation "-90.000000,180.000000,0.000000")))
        (Class|ControlRigComponent|SetControlTransform (Variables|Default|GetControlRig) (Utilities|String|StringToName _array_element) (Math|Transform|MakeTransform (* (.Value (Utilities|Map|Find _posedata _array_element)) "100.000000,100.000000,100.000000") _output_get "0.000000,0.000000,0.000000") "RigSpace") ; Update control rig programmatically
      ))))

(fn ConstructionScript)